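; Checkerboard tile actor for the map, showing a galaxy model and tracking the units standing on it through box overlap.
; Construction picks a random name from a data table; clicking moves the player controller's board selection here and opens a building UI, if a board was already selected.
; Tick drives material and visibility updates from the board data component, plus a delayed change check that re-initialises building slots.
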(event OnComponentBeginOverlap(Box)
  (params (OverlappedComponent :type Primitive%20Component%20Object%20Reference) (OtherActor :type Actor%20Object%20Reference) (OtherComp :type Primitive%20Component%20Object%20Reference) (OtherBodyIndex :type Integer) (bFromSweep :type Boolean) (SweepResult :type Hit%20Result%20Structure%20%28by%20ref%29))
  ;[1 1 1] 将unit从board中添加或移除
  (Utilities|Casting|CastToBP_BaseUnit OtherActor)
  (Utilities|Array|Add (Variables|/Game/BluePrint/MapSystem/BuildingSlot/BPC_CheckBoardUnitSystem.BPC_CheckBoardUnitSystem_C|GetUnitContains (Variables|Default|GetBPC_UnitSystem)) 0))

(event OnComponentEndOverlap(Box)
  (params (OverlappedComponent :type Primitive%20Component%20Object%20Reference) (OtherActor :type Actor%20Object%20Reference) (OtherComp :type Primitive%20Component%20Object%20Reference) (OtherBodyIndex :type Integer))
  ;[1 1 1] 将unit从board中添加或移除
  (bind _asbp_base_unit (Utilities|Casting|CastToBP_BaseUnit OtherActor))
  (Utilities|Array|RemoveItem (Variables|/Game/BluePrint/MapSystem/BuildingSlot/BPC_CheckBoardUnitSystem.BPC_CheckBoardUnitSystem_C|GetUnitContains (Variables|Default|GetBPC_UnitSystem)) _asbp_base_unit))

(event OnClicked(CheckBoard)
  (params (TouchedComponent :type Primitive%20Component%20Object%20Reference) (ButtonPressed :type Key%20Structure :default "None"))
  ;[1 1 1] 左键单击设置选中的Unit与board
  (bind _asbp_player_controller (Utilities|Casting|CastToBP_PlayerController (Game|GetPlayerController 0)))
  (Variables|/Game/BluePrint/Player/PlayerController/BP_PlayerController.BP_PlayerController_C|SetSelectedUnit _asbp_player_controller 0)
  (bind _currentselectedboard (Variables|/Game/BluePrint/Player/PlayerController/BP_PlayerController.BP_PlayerController_C|GetCurrentSelectedBoard _asbp_player_controller)
    (:then
      (Variables|/Game/BluePrint/MapSystem/MapData/BPC_checkBoardData.BPC_checkBoardData_C|SetChoosed (Variables|BP_checkerboard_C|GetBPC_checkBoardData _currentselectedboard) false)
      (Variables|/Game/BluePrint/Player/PlayerController/BP_PlayerController.BP_PlayerController_C|SetCurrentSelectedBoard _asbp_player_controller self)
      (Variables|/Game/BluePrint/MapSystem/MapData/BPC_checkBoardData.BPC_checkBoardData_C|SetChoosed (Variables|Default|GetBPC_checkBoardData) true)
      ;[1 1 1] 添加buildingUI
      (bind _asbp_player_controller_2 (Utilities|Casting|CastToBP_PlayerController (Game|GetPlayerController 0)))
      (bind _returnvalue (UserInterface|CreateWidget "/Game/BluePrint/Wiget/BuildingWidgt/W_BuildingUI.W_BuildingUI_C" _asbp_player_controller_2 self))
      (bind _output_get (Variables|/Game/BluePrint/Player/PlayerController/BP_PlayerController.BP_PlayerController_C|SetBuildingUI _asbp_player_controller_2 _returnvalue))
      (UserInterface|Viewport|AddtoViewport _output_get 0))
    (:else)))

(event EventTick
  (params (DeltaSeconds :type Float%20%28single-precision%29))
  (Utilities|SetcheckBoardColor)
  (Utilities|InitBoard))

(fn ConstructionScript
  (bind _returnvalue (Utilities|GetDataTableRow "/Game/BluePrint/Data/PlayData/Maps/DT_CheckBoardName.DT_CheckBoardName" (Utilities|String|StringToName (Utilities|String|ToString(Integer) (Math|Random|RandomIntegerinRange 0 10))))
    (:then
      (Variables|Default|SetName (.name _returnvalue)))))

(fn SetColor
  (params (Material :type Material%20Interface%20Object%20Reference) (目标 :type Primitive%20Component%20Object%20Reference))
  (Rendering|Material|SetMaterial 目标 0 Material))

(fn Discovered)

(fn Init
  (bind _bpc_checkboard_buildingslot (Variables|Default|GetBPC_checkboard_BuildingSlot))
  (Default|Init _bpc_checkboard_buildingslot)
  (Variables|/Game/BluePrint/MapSystem/MapData/BPC_checkBoardData.BPC_checkBoardData_C|SetSlotNum (Variables|Default|GetBPC_checkBoardData) (Variables|/Game/BluePrint/MapSystem/BuildingSlot/BPC_checkboard_BuildingSlot.BPC_checkboard_BuildingSlot_C|GetSlotNum _bpc_checkboard_buildingslot)))