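; Player controller for a turn-based board game that builds the player HUD and handles right-click movement of the selected unit.
; BeginPlay creates the play and side-info widgets, then assigns every checkerboard tile to the player state as a test.
; Right-click traces under the cursor and AI-moves the unit to a usable, shown tile, clearing old neighbour highlights.
; Once the move is issued, it spends unit power and refreshes tile, unit list and neighbours; the player Energy check gates nothing.
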(event EventBeginPlay
  (bind _self self)
  (bind _astest_player_pawn (Utilities|Casting|CastToTest_Player_Pawn (Game|Player|GetPlayerPawn 0)))
  (bind _returnvalue (UserInterface|CreateWidget "/Game/BluePrint/Wiget/PlayWidget/W_Play.W_Play_C" _self _astest_player_pawn))
  (bind _returnvalue_2 (UserInterface|CreateWidget "/Game/BluePrint/Wiget/Player_RightSide_Info.Player_RightSide_Info_C" _self))
  (UserInterface|Viewport|AddtoViewport _returnvalue_2 0)
  (Variables|Default|SetRightSideInfo _returnvalue_2)
  ;[1 1 1] 用来测试折叠控件
  (bind _outactors (Actor|GetAllActorsOfClass "/Game/BluePrint/MapSystem/BP_checkerboard.BP_checkerboard_C"))
  (for _array_element _outactors
    (Utilities|Array|Add (Variables|/Game/BluePrint/Player/PlayerController/BPC_PlayerData.BPC_PlayerData_C|GetCheckBoardOwned (Variables|/Game/BluePrint/Manager/GameModeManager/GM_TurnBasePlayerState.GM_TurnBasePlayerState_C|GetBPC_PlayerData (.AsGM%20Turn%20Base%20Player%20State (Utilities|Casting|CastToGM_TurnBasePlayerState (Variables|/Script/Engine.Pawn|GetPlayerState (.AsTest%20Player%20Pawn (Utilities|Casting|CastToTest_Player_Pawn (Game|Player|GetPlayerPawn 0)))))))) _array_element))
  (Default|RefreshCheckBoards (Variables|Default|GetRightSideInfo)))

(event EventTick
  (params (DeltaSeconds :type Float%20%28single-precision%29)))

(event Input|MouseEvents|RightMouseButton
  (params (Key :type Key%20Structure :default "None"))
  (bind _returnvalue (Game|GetPlayerCameraManager 0))
  (bind _rootcomponent (Variables|/Script/Engine.Actor|GetRootComponent _returnvalue))
  (bind _returnvalue_2 (Transformation|GetWorldLocation _rootcomponent))
  ;[1 1 1] 右键单击，被选中的单位移动
  (:Pressed
    (bind (_outhit _returnvalue_3) (Collision|LineTraceByChannel _returnvalue_2 (+ _returnvalue_2 (* (.WorldDirection (Game|Player|ConvertMouseLocationToWorldSpace (Game|GetPlayerController 0))) 1e+08)) "TraceTypeQuery1" false 0 "None"))
    (if _returnvalue_3
      (bind _asbp_checkerboard (Utilities|Casting|CastToBP_checkerboard (.HitActor (Collision|BreakHitResult _outhit))))
      (bind _selectedunit (Variables|Default|GetSelectedUnit)
        (:then
          (if (> (Variables|/Game/BluePrint/Player/PlayerController/BPC_PlayerData.BPC_PlayerData_C|GetEnergy (Variables|/Game/BluePrint/Manager/GameModeManager/GM_TurnBasePlayerState.GM_TurnBasePlayerState_C|GetBPC_PlayerData (.AsGM%20Turn%20Base%20Player%20State (Utilities|Casting|CastToGM_TurnBasePlayerState (Variables|GetPlayerState))))) 0)
            _
            (else
              _))
          (if (Variables|/Game/BluePrint/MapSystem/MapData/BPC_checkBoardData.BPC_checkBoardData_C|GetUseable (Variables|/Game/BluePrint/MapSystem/BP_checkerboard.BP_checkerboard_C|GetBPC_checkBoardData _asbp_checkerboard))
            (if (Variables|/Game/BluePrint/MapSystem/BP_checkerboard.BP_checkerboard_C|GetShowed? _asbp_checkerboard)
              (for _array_element (Variables|/Game/BluePrint/MapSystem/BP_checkerboard.BP_checkerboard_C|GetNeighbours (Variables|/Game/BluePrint/Player/Unit/BP_BaseUnit.BP_BaseUnit_C|GetCurrentBoard (Variables|Default|GetSelectedUnit)))
                (Variables|/Game/BluePrint/MapSystem/BP_checkerboard.BP_checkerboard_C|SetShowed? _array_element false))
              (AI|AIMoveTo _selectedunit "0, 0, 0" _asbp_checkerboard 0.0 false
                (:then
                  (Default|CostPower (Variables|Default|GetSelectedUnit))
                  (Default|Refresh _asbp_checkerboard)
                  (Utilities|FlowControl|Delay 0.5)
                  ;[1 0.06016 0.1658] 刷新单位列表
                  (bind _foundwidgets (Widget|GetAllWidgetsOfClass "/Game/BluePrint/Wiget/BuildingWidgt/W_BuildingUI.W_BuildingUI_C" true))
                  (Default|RefreshUnits (Utilities|Array|Get(acopy) _foundwidgets))
                  (Default|ShowNeighbour _asbp_checkerboard))))))
        (:else)))))

(fn ConstructionScript)