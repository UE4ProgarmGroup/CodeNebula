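; BP_BuildingSlot is a map-system building slot that randomly picks its building kind.
; The Construction Script runs a cascade of independent random rolls with rising thresholds, selecting one of five enum kinds with heavy bias toward the first.
; Every branch sets BuildingImage to None, and the event graph has no active logic.
; Because the roll happens at construction, the kind can change whenever the script reruns.
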(event EventBeginPlay)

(event Collision|EventActorBeginOverlap
  (params (OtherActor :type Actor%20Object%20Reference)))

(event EventTick
  (params (DeltaSeconds :type Float%20%28single-precision%29)))

(fn ConstructionScript
  (bind _returnvalue (Math|Random|RandomFloatinRange 0.0 1e+02))
  (if (< _returnvalue 6e+01)
    (Variables|Default|SetKind "NewEnumerator0")
    (Variables|Default|SetBuildingImage 0)
    (elif (< _returnvalue 8e+01)
      (Variables|Default|SetKind "NewEnumerator1")
      (Variables|Default|SetBuildingImage 0)
      (elif (< _returnvalue 9e+01)
        (Variables|Default|SetKind "NewEnumerator2")
        (Variables|Default|SetBuildingImage 0)
        (elif (< _returnvalue 95.0)
          (Variables|Default|SetKind "NewEnumerator3")
          (Variables|Default|SetBuildingImage 0)
          (else
            (Variables|Default|SetKind "NewEnumerator4")
            (Variables|Default|SetBuildingImage 0)))))))