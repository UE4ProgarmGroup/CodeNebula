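; BP_Building is a player-owned building actor, apparently a base for buildable structures, that handles resource cost and refund.
; Cost subtracts its material and energy costs from the owner's BPCPlayerData component.
; Dismantle adds a separate Material value back to the owner, without refunding energy, then destroys the actor.
; Action and Service are empty functions, and the event graph and construction script contain no logic.
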(event EventBeginPlay)

(event Collision|EventActorBeginOverlap
  (params (OtherActor :type Actor%20Object%20Reference)))

(event EventTick
  (params (DeltaSeconds :type Float%20%28single-precision%29)))

(event EventDestroyed)

(fn ConstructionScript)

(fn Action)

(fn Service)

(fn Cost
  (bind _playerowner (Variables|Default|GetPlayerOwner))
  (bind _bpc_playerdata (Variables|/Game/BluePrint/Player/PlayerController/Test_Player_Pawn.Test_Player_Pawn_C|GetBPC_PlayerData _playerowner))
  (Variables|/Game/BluePrint/Player/PlayerController/BPC_PlayerData.BPC_PlayerData_C|SetMeterial _bpc_playerdata (- (Variables|/Game/BluePrint/Player/PlayerController/BPC_PlayerData.BPC_PlayerData_C|GetMeterial _bpc_playerdata) (Variables|消耗值|GetMeterialCost)))
  (Variables|/Game/BluePrint/Player/PlayerController/BPC_PlayerData.BPC_PlayerData_C|SetEnergy _bpc_playerdata (- (Variables|/Game/BluePrint/Player/PlayerController/BPC_PlayerData.BPC_PlayerData_C|GetEnergy _bpc_playerdata) (Variables|消耗值|GetEnergyCost))))

(fn Dismantle
  (bind _playerowner (Variables|Default|GetPlayerOwner))
  (bind _bpc_playerdata (Variables|/Game/BluePrint/Player/PlayerController/Test_Player_Pawn.Test_Player_Pawn_C|GetBPC_PlayerData _playerowner))
  (Variables|/Game/BluePrint/Player/PlayerController/BPC_PlayerData.BPC_PlayerData_C|SetMeterial _bpc_playerdata (+ (Variables|产出值|GetMaterial) (Variables|/Game/BluePrint/Player/PlayerController/BPC_PlayerData.BPC_PlayerData_C|GetMeterial _bpc_playerdata)))
  (Actor|DestroyActor))