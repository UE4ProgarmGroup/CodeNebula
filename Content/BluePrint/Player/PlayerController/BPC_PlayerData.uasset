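; BPC_PlayerData is a player data component that tracks owned buildings and the resources they provide.
; Tick runs through a one-second Delay into BuildingRefresh, so totals update periodically rather than every frame.
; BuildingRefresh resets and re-sums per-round energy and material, plus science points, from every entry in BuildingOwned.
; BuildingAwake separately calls Action on each owned building and is not invoked within this graph.
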(event EventBeginPlay)

(event EventTick
  (params (DeltaSeconds :type Float%20%28single-precision%29))
  (Utilities|FlowControl|Delay 1.0)
  (CallFunction|BuildingRefresh))

(fn BuildingAwake
  (for _array_element (Variables|单位|GetBuildingOwned)
    (Default|Action _array_element)))

(fn BuildingRefresh
  (Variables|资源|SetSciencePoint 0)
  (Variables|资源|SetEnergyEveryRound 0)
  (Variables|资源|SetMeterialEveryRound 0)
  (for _array_element (Variables|单位|GetBuildingOwned)
    (Variables|资源|SetEnergyEveryRound (+ (Variables|资源|GetEnergyEveryRound) (Variables|/Game/BluePrint/Player/Building/BP_Building.BP_Building_C|GetEnergy _array_element)))
    (Variables|资源|SetMeterialEveryRound (+ (Variables|资源|GetMeterialEveryRound) (Variables|/Game/BluePrint/Player/Building/BP_Building.BP_Building_C|GetMaterial _array_element)))
    (Variables|资源|SetSciencePoint (+ (Variables|资源|GetSciencePoint) (Variables|/Game/BluePrint/Player/Building/BP_Building.BP_Building_C|GetSciencePoint _array_element)))))