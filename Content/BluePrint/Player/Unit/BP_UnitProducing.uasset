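; BP_UnitProducing is an actor that represents a unit in production on a CheckBoard and turns into that unit when enough work accumulates.
; Its construction script takes the required work from UnitProducing, and Work adds the board's building-slot WorkNum to the running total.
; Tick, throttled by a half-second Delay, calls Produce, which spawns the unit once work exceeds the requirement, registers it with the board's unit system and destroys itself.
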(event EventBeginPlay)

(event Collision|EventActorBeginOverlap
  (params (OtherActor :type Actor%20Object%20Reference)))

(event EventTick
  (params (DeltaSeconds :type Float%20%28single-precision%29))
  (Utilities|FlowControl|Delay 0.5)
  (CallFunction|Produce))

(fn ConstructionScript
  (Variables|Default|SetWorksNeeded (.works (Variables|Default|GetUnitProducing))))

(fn Produce
  (if (> (Variables|Default|GetWorks) (Variables|Default|GetWorksNeeded))
    (bind _returnvalue (Game|SpawnActorfromClass (.unitclass (Variables|Default|GetUnitProducing)) (Transformation|GetActorTransform) "Undefined" 0 0))
    (Utilities|Array|Add (Variables|/Game/BluePrint/MapSystem/BuildingSlot/BPC_CheckBoardUnitSystem.BPC_CheckBoardUnitSystem_C|GetUnitContains (Variables|/Game/BluePrint/MapSystem/BP_checkerboard.BP_checkerboard_C|GetBPC_UnitSystem (Variables|Default|GetCheckBoard))) _returnvalue)
    (Actor|DestroyActor)))

(fn Work
  (Variables|Default|SetWorks (+ (Variables|Default|GetWorks) (Variables|/Game/BluePrint/MapSystem/BuildingSlot/BPC_checkboard_BuildingSlot.BPC_checkboard_BuildingSlot_C|GetWorkNum (Variables|/Game/BluePrint/MapSystem/BP_checkerboard.BP_checkerboard_C|GetBPC_checkboard_BuildingSlot (Variables|Default|GetCheckBoard))))))