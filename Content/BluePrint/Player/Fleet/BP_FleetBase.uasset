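; Base fleet actor that groups player units for selection, movement, scanning, merging and attacking in a turn-based board game.
; FleetMove sends units by AI MoveTo to the controller's Destination if it is usable, shown and energy remains, charging move energy.
; Scans read the first unit's board to fill the fleet controller with ally or enemy widgets.
; Merge reassigns units' fleet and destroys the other; attack pairs each unit with a random enemy.
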(event Custom|FleetMove
  (for _array_element (Variables|Default|GetUnits)
    (bind _destination (Variables|/Game/BluePrint/Player/PlayerController/BP_PlayerController.BP_PlayerController_C|GetDestination (.AsBP%20Player%20Controller (Utilities|Casting|CastToBP_PlayerController (Game|GetPlayerController 0))))
      (:then
        (if (> (Variables|/Game/BluePrint/Player/PlayerController/BPC_PlayerData.BPC_PlayerData_C|GetEnergy (Variables|/Game/BluePrint/Manager/GameModeManager/GM_TurnBasePlayerState.GM_TurnBasePlayerState_C|GetBPC_PlayerData (.AsGM%20Turn%20Base%20Player%20State (Utilities|Casting|CastToGM_TurnBasePlayerState (Variables|/Script/Engine.Pawn|GetPlayerState (Game|Player|GetPlayerPawn 0)))))) 0)
          (if (Variables|/Game/BluePrint/MapSystem/MapData/BPC_checkBoardData.BPC_checkBoardData_C|GetUseable (Variables|/Game/BluePrint/MapSystem/BP_checkerboard.BP_checkerboard_C|GetBPC_checkBoardData _destination))
            (if (Variables|/Game/BluePrint/MapSystem/BP_checkerboard.BP_checkerboard_C|GetShowed? _destination)
              (AI|AIMoveTo _array_element "0, 0, 0" _destination 5.0 false
                (:then
                  (Default|CostPower _array_element (Variables|/Game/BluePrint/Player/Unit/BP_BaseUnit.BP_BaseUnit_C|GetMoveEnergyCost _array_element))))))))
      (:else)))
  (Default|Refresh _destination)
  (bind _foundwidgets (Widget|GetAllWidgetsOfClass "/Game/BluePrint/Wiget/BuildingWidgt/W_BuildingUI.W_BuildingUI_C" true))
  (Default|RefreshUnits (Utilities|Array|Get(acopy) _foundwidgets))
  (Default|RefreFleets (Utilities|Array|Get(acopy) _foundwidgets)))

(event Custom|FleetAttack
  (params (FleetToAttack :type BP%20Fleet%20Base%20Object%20Reference))
  (Utilities|Array|Clear (Variables|Default|GetEnermyUnits))
  (Variables|Default|SetEnermyUnits (Variables|BP_FleetBase_C|GetUnits FleetToAttack))
  (for _array_element (Variables|Default|GetUnits)
    (Default|Attack _array_element (.OutItem (Utilities|Array|Random (Variables|Default|GetEnermyUnits))))))

(event Custom|FleetScanAlly
  (params (FleetController :type W%20Fleet%20Controller%20Object%20Reference))
  (bind _units (Variables|Default|GetUnits))
  (bind _fleetbox (Variables|/Game/BluePrint/Wiget/FleetWidget/W_FleetController.W_FleetController_C|GetFleetBox FleetController))
  (bind _output (Utilities|Array|Get(acopy) _units))
  (Utilities|Array|Clear (Variables|Default|GetAlies))
  (Widget|Panel|ClearChildren _fleetbox)
  (for _array_element (Variables|/Game/BluePrint/MapSystem/BuildingSlot/BPC_CheckBoardUnitSystem.BPC_CheckBoardUnitSystem_C|GetFleetContains (Variables|/Game/BluePrint/MapSystem/BP_checkerboard.BP_checkerboard_C|GetBPC_UnitSystem (Variables|/Game/BluePrint/Player/Unit/BP_BaseUnit.BP_BaseUnit_C|GetCurrentBoard _output)))
    (if (not (!= _array_element self))
      (if (== (Variables|BP_FleetBase_C|Getnum _array_element) (Variables|/Game/BluePrint/Player/Unit/BP_BaseUnit.BP_BaseUnit_C|GetPlayerNum _output))
        (Utilities|Array|Add (Variables|Default|GetAlies) 0)
        (bind _returnvalue (UserInterface|CreateWidget "/Game/BluePrint/Wiget/W_AllyFleets.W_AllyFleets_C" (Game|GetPlayerController 0) _array_element self FleetController))
        (Widget|Panel|AddChild _fleetbox _returnvalue)))))

(event Custom|FleetScanEnermy
  (params (FleetController :type W%20Fleet%20Controller%20Object%20Reference))
  (bind _fleetbox (Variables|/Game/BluePrint/Wiget/FleetWidget/W_FleetController.W_FleetController_C|GetFleetBox FleetController))
  (bind _units (Variables|Default|GetUnits))
  (bind _output (Utilities|Array|Get(acopy) _units))
  (Utilities|Array|Clear (Variables|Default|GetEnermyFleets))
  (Widget|Panel|ClearChildren _fleetbox)
  (for _array_element (Variables|/Game/BluePrint/MapSystem/BuildingSlot/BPC_CheckBoardUnitSystem.BPC_CheckBoardUnitSystem_C|GetFleetContains (Variables|/Game/BluePrint/MapSystem/BP_checkerboard.BP_checkerboard_C|GetBPC_UnitSystem (Variables|/Game/BluePrint/Player/Unit/BP_BaseUnit.BP_BaseUnit_C|GetCurrentBoard _output)))
    (if (!= (Variables|BP_FleetBase_C|Getnum _array_element) (Variables|/Game/BluePrint/Player/Unit/BP_BaseUnit.BP_BaseUnit_C|GetPlayerNum _output))
      (Utilities|Array|Add (Variables|Default|GetEnermyFleets) _array_element)
      (bind _returnvalue (UserInterface|CreateWidget "/Game/BluePrint/Wiget/W_EnermyFleets.W_EnermyFleets_C" (Game|GetPlayerController 0) _array_element self))
      (Widget|Panel|AddChild _fleetbox _returnvalue))))

(event Custom|FleetMerge
  (params (FleetToMerge :type BP%20Fleet%20Base%20Object%20Reference))
  (bind _units (Variables|BP_FleetBase_C|GetUnits FleetToMerge))
  (for _array_element _units
    (Variables|/Game/BluePrint/Player/Unit/BP_BaseUnit.BP_BaseUnit_C|SetFleet _array_element self)
    (if (not (Utilities|Array|ContainsItem _units _array_element))
      (Utilities|Array|Add (Variables|Default|GetUnits) _array_element)
      (Development|PrintString "addUnit")))
  (Actor|DestroyActor FleetToMerge)
  (Development|PrintString "Destroyed"))

(fn ConstructionScript)

(fn SelectFleet
  (Variables|/Game/BluePrint/Player/PlayerController/BP_PlayerController.BP_PlayerController_C|SetSelectedFleet (.AsBP%20Player%20Controller (Utilities|Casting|CastToBP_PlayerController (Game|GetPlayerController 0))) self)
  (bind _foundwidgets (Widget|GetAllWidgetsOfClass "/Game/BluePrint/Wiget/FleetWidget/W_FleetController.W_FleetController_C" false))
  (for _array_element _foundwidgets
    (Widget|RemovefromParent _array_element))
  (bind _returnvalue (UserInterface|CreateWidget "/Game/BluePrint/Wiget/FleetWidget/W_FleetController.W_FleetController_C" (Game|GetPlayerController 0)))
  (UserInterface|Viewport|AddtoViewport _returnvalue 0))