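; Turn-based GameState that cycles turns through the PlayerArray and counts rounds, with the player count cached in the construction script.
; NewTurn enables cursor, click and touch input on the current player's BP_PlayerController, found by using the player state's PlayerId as the controller index.
; EndNewTurn disables that input and advances the turn, calling NewRound to increment the round and restart at the first player after the last one.
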(event EventBeginPlay)

(event EventTick
  (params (DeltaSeconds :type Float%20%28single-precision%29)))

(fn ConstructionScript
  (Variables|Default|SetPlayerNum (Utilities|Array|Length (Variables|Default|GetPlayerArray))))

(fn NewTurn
  (bind _asgm_turn_base_player_state (Utilities|Casting|CastToGM_TurnBasePlayerState (Utilities|Array|Get(acopy) (Variables|Default|GetPlayerArray) (Variables|Default|GetTurns))))
  (bind _asbp_player_controller (Utilities|Casting|CastToBP_PlayerController (Game|GetPlayerController (Variables|/Script/Engine.PlayerState|GetPlayerId _asgm_turn_base_player_state))))
  (Variables|/Script/Engine.PlayerController|SetbShowMouseCursor _asbp_player_controller true)
  (Variables|/Script/Engine.PlayerController|SetbEnableClickEvents _asbp_player_controller true)
  (Variables|/Script/Engine.PlayerController|SetbEnableTouchEvents _asbp_player_controller true))

(fn EndNewTurn
  (bind _asgm_turn_base_player_state (Utilities|Casting|CastToGM_TurnBasePlayerState (Utilities|Array|Get(acopy) (Variables|Default|GetPlayerArray) (Variables|Default|GetTurns))))
  (bind _asbp_player_controller (Utilities|Casting|CastToBP_PlayerController (Game|GetPlayerController (Variables|/Script/Engine.PlayerState|GetPlayerId _asgm_turn_base_player_state))))
  (Variables|/Script/Engine.PlayerController|SetbShowMouseCursor _asbp_player_controller false)
  (Variables|/Script/Engine.PlayerController|SetbEnableClickEvents _asbp_player_controller false)
  (Variables|/Script/Engine.PlayerController|SetbEnableTouchEvents _asbp_player_controller false)
  (Math|Integer|IncrementInt (Variables|Default|GetTurns)
    (:%20%20
      (if (>= (Variables|Default|GetTurns) (Variables|Default|GetPlayerNum))
        (CallFunction|NewRound)
        (else
          (CallFunction|NewTurn))))))

(fn NewRound
  (Math|Integer|IncrementInt (Variables|Default|GetRounds)
    (:%20%20
      (Variables|Default|SetTurns 0)
      (CallFunction|NewTurn))))