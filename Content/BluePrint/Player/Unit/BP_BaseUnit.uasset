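; BP_BaseUnit is the base unit for a turn-based board game, handling selection, movement, attacks and damage.
; On BeginPlay it spawns its own fleet actor and registers itself in it.
; Moves AI-walk to the player controller's destination tile if shown, usable and energy remains, then refresh tiles and UI.
; Moves and attacks deduct player-state energy; selection opens an options widget, and the unit is destroyed when life runs out.
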(event Custom|Unit_Move
  ;[1 1 1] 单位移动
  (CallFunction|UnitMoveonClient))

(event Custom|UnitMove_OnClient
  (bind _self self)
  ;[1 1 1] 单位移动
  (bind _destination (Variables|/Game/BluePrint/Player/PlayerController/BP_PlayerController.BP_PlayerController_C|GetDestination (.AsBP%20Player%20Controller (Utilities|Casting|CastToBP_PlayerController (Game|GetPlayerController 0))))
    (:then
      (if (> (Variables|/Game/BluePrint/Player/PlayerController/BPC_PlayerData.BPC_PlayerData_C|GetEnergy (Variables|/Game/BluePrint/Manager/GameModeManager/GM_TurnBasePlayerState.GM_TurnBasePlayerState_C|GetBPC_PlayerData (.AsGM%20Turn%20Base%20Player%20State (Utilities|Casting|CastToGM_TurnBasePlayerState (Variables|/Script/Engine.Pawn|GetPlayerState (Game|Player|GetPlayerPawn 0)))))) 0)
        (if (Variables|/Game/BluePrint/MapSystem/MapData/BPC_checkBoardData.BPC_checkBoardData_C|GetUseable (Variables|/Game/BluePrint/MapSystem/BP_checkerboard.BP_checkerboard_C|GetBPC_checkBoardData _destination))
          (if (Variables|/Game/BluePrint/MapSystem/BP_checkerboard.BP_checkerboard_C|GetShowed? _destination)
            (for _array_element (Variables|/Game/BluePrint/MapSystem/BP_checkerboard.BP_checkerboard_C|GetNeighbours (Variables|BP_BaseUnit_C|GetCurrentBoard _self))
              (Variables|/Game/BluePrint/MapSystem/BP_checkerboard.BP_checkerboard_C|SetShowed? _array_element false))
            (AI|AIMoveTo _self "0, 0, 0" _destination 5.0 false
              (:then
                (CallFunction|CostPower _self (Variables|Default|GetMoveEnergyCost))
                (Default|Refresh _destination)
                ;;[1 0.06016 0.1658] 刷新单位列表,舰队列表
                (bind _foundwidgets (Widget|GetAllWidgetsOfClass "/Game/BluePrint/Wiget/BuildingWidgt/W_BuildingUI.W_BuildingUI_C" true))
                (Default|RefreshUnits (Utilities|Array|Get(acopy) _foundwidgets))
                (Default|RefreFleets (Utilities|Array|Get(acopy) _foundwidgets))
                (Default|ShowNeighbour _destination)))))))
    (:else)))

(event Game|Damage|EventAnyDamage
  (params (Damage :type Float%20%28single-precision%29) (DamageType :type Damage%20Type%20Object%20Reference) (InstigatedBy :type Controller%20Object%20Reference) (DamageCauser :type Actor%20Object%20Reference))
  ;[1 1 1] 被攻击
  (bind _output_get (Variables|Default|SetUnitLife (- (Variables|Default|GetUnitLife) Damage)))
  (if (<= _output_get 0.0)
    (Actor|DestroyActor)))

(event EventBeginPlay
  (bind _returnvalue (Game|SpawnActorfromClass "/Game/BluePrint/Player/Fleet/BP_FleetBase.BP_FleetBase_C" (Math|Transform|MakeTransform "0, 0, 0") "Undefined" 0 0 0))
  (bind _output_get (Variables|Default|SetFleet _returnvalue))
  (Variables|/Game/BluePrint/Player/Fleet/BP_FleetBase.BP_FleetBase_C|Setnum _output_get (Variables|Default|GetPlayerNum))
  (Utilities|Array|Add (Variables|/Game/BluePrint/Player/Fleet/BP_FleetBase.BP_FleetBase_C|GetUnits _output_get) self))

(fn ConstructionScript)

(fn CostPower
  (params (EnergyCost :type Integer))
  (bind _astest_player_pawn (Utilities|Casting|CastToTest_Player_Pawn (Game|Player|GetPlayerPawn 0)))
  (Variables|/Game/BluePrint/Player/PlayerController/BPC_PlayerData.BPC_PlayerData_C|SetEnergy (Variables|/Game/BluePrint/Manager/GameModeManager/GM_TurnBasePlayerState.GM_TurnBasePlayerState_C|GetBPC_PlayerData (.AsGM%20Turn%20Base%20Player%20State (Utilities|Casting|CastToGM_TurnBasePlayerState (Variables|/Script/Engine.Pawn|GetPlayerState _astest_player_pawn)))) (- (Variables|/Game/BluePrint/Player/PlayerController/BPC_PlayerData.BPC_PlayerData_C|GetEnergy (Variables|/Game/BluePrint/Manager/GameModeManager/GM_TurnBasePlayerState.GM_TurnBasePlayerState_C|GetBPC_PlayerData (.AsGM%20Turn%20Base%20Player%20State (Utilities|Casting|CastToGM_TurnBasePlayerState (Variables|/Script/Engine.Pawn|GetPlayerState _astest_player_pawn))))) EnergyCost)))

(fn SelectUnit
  (bind _asbp_player_controller (Utilities|Casting|CastToBP_PlayerController (Game|GetPlayerController 0)))
  (Variables|/Game/BluePrint/Player/PlayerController/BP_PlayerController.BP_PlayerController_C|SetSelectedUnit _asbp_player_controller self)
  (Development|PrintString "selected")
  (bind _foundwidgets (Widget|GetAllWidgetsOfClass "/Game/BluePrint/Wiget/W_UnitOptions.W_UnitOptions_C" false))
  (for _array_element _foundwidgets
    (Widget|RemovefromParent _array_element))
  (bind _returnvalue (UserInterface|CreateWidget "/Game/BluePrint/Wiget/W_UnitOptions.W_UnitOptions_C" (Game|GetPlayerController 0) self))
  (UserInterface|Viewport|AddtoViewport _returnvalue 0))

(fn Attack
  (params (AttackedEnermy :type BP%20Base%20Unit%20Object%20Reference))
  (Game|Damage|ApplyDamage AttackedEnermy (Variables|Default|GetUnitDamage) 0 0)
  (CallFunction|CostPower (Variables|Default|GetAttackEnergyCost)))